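; Enemy AI pawn that attacks the player and dies when its health runs out.
; Attack turns it toward the player and plays a montage while a timeline drives a red camera fade, then fires OnAttackFinished on completion.
; The attack applies no damage here, only the screen effect.
; AnyDamage reduces health and, at zero, plays a death montage once before unpossessing the AI controller.
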(event `Attack`
  (`self.K2_SetActorRotation` (`KismetMathLibrary.FindLookAtRotation` (`self.K2_GetActorLocation`) (`self.K2_GetActorLocation` (`GameplayStatics.GetPlayerPawn` 0))))
  (`|PlayMontage` (`self.Mesh`) "/Game/AI/Character/Animations/AM_Attack.AM_Attack"
    (:`then`
      (bind (_direction _newtrack_0) (`Timeline|Timeline_0` :!via `PlayFromStart`)
        (:`Update`
          (`PlayerCameraManager.SetManualCameraFade` (`PlayerController.PlayerCameraManager` (`GameplayStatics.GetPlayerController` 0)) _newtrack_0 (struct :`R` 1.0 :`A` 0.6) false))))
    (:`OnCompleted`
      (`self.OnAttackFinished`))))

(event `self.ReceiveAnyDamage`
  (params (Damage :type "Float (single-precision)") (DamageType :type "DamageType Object Reference") (InstigatedBy :type "Controller Object Reference") (DamageCauser :type "Actor Object Reference"))
  (if (> (`self.HealthValue`) 0.0)
    (bind _output_get (set `self.HealthValue` (- (`self.HealthValue`) Damage)))
    (if (<= _output_get 0.0)
      (`/Engine/EditorBlueprintResources/StandardMacros.DoOnce` false
        (:`Completed`
          (`|PlayMontage` (`self.Mesh`) "/Game/AI/Character/Animations/AM_Dead.AM_Dead"
            (:`OnCompleted`
              (`Controller.UnPossess` (`AIBlueprintHelperLibrary.GetAIController` self)))))))))

(fn `UserConstructionScript`)