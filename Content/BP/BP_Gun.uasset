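; BP_Gun is a gun actor that BP_MotionController picks up, drops and fires.
; Pickup disables mesh physics, attaches the gun and eases it into place; Drop detaches it and restores physics.
; While held, Shoot plays fire effects and line-traces along the Nozzle socket's forward vector, with the end point not offset from the muzzle.
; Hits spawn a decal and impact emitter, send an impulse message and apply damage.
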(event `/Game/VirtualRealityBP/Blueprints/PickupActorInterface.Pickup`
  (params (AttachTo :type "SceneComponent Object Reference"))
  (bind _returnvalue (`self.K2_GetRootComponent`))
  (`PrimitiveComponent.SetSimulatePhysics` (`self.gun_mesh`) false)
  (`SceneComponent.K2_AttachToComponent` _returnvalue AttachTo "None" "KeepWorld" "KeepWorld" "KeepWorld" false)
  (`KismetSystemLibrary.MoveComponentTo` _returnvalue (-4.0 0.0 -1.0))
  (set `self.IsHeld` true))

(event `/Game/VirtualRealityBP/Blueprints/PickupActorInterface.Drop`
  (`PrimitiveComponent.SetSimulatePhysics` (`self.gun_mesh`) true)
  (`self.K2_DetachFromActor` "KeepWorld" "KeepWorld" "KeepWorld")
  (set `self.IsHeld` false))

(event `/Game/VirtualRealityBP/Blueprints/BPI_Gun.Shoot`
  (bind _gun_mesh (`self.gun_mesh`))
  (bind (_returnvalue_location _returnvalue_rotation) (`KismetMathLibrary.BreakTransform` (`SceneComponent.GetSocketTransform` _gun_mesh "Nozzle" "RTS_World")))
  (bind _returnvalue (`KismetMathLibrary.GetForwardVector` _returnvalue_rotation))
  (if (`self.IsHeld`)
    (`SkeletalMeshComponent.PlayAnimation` _gun_mesh "/Game/Models/Pistol/Animations/ANIM_G18_Fire.ANIM_G18_Fire" false)
    (`GameplayStatics.SpawnEmitterAtLocation` null _returnvalue_location _returnvalue_rotation)
    (`GameplayStatics.PlaySoundAtLocation` "/Game/Audio/Weapon_AssaultRifle/AK_47/SC_Gun.SC_Gun" _returnvalue_location (struct) 1.0 1.0 0.0 null null null null)
    (bind (_outhit _returnvalue_2) (`KismetSystemLibrary.LineTraceSingle` :`Start` _returnvalue_location :`End` (* _returnvalue 100000.0) :`TraceChannel` "TraceTypeQuery1" :`DrawDebugType` "ForDuration"))
    (if _returnvalue_2
      (bind (_bblockinghit _binitialoverlap _time _distance _location _impactpoint _normal _impactnormal _physmat _hitactor _hitcomponent) (`GameplayStatics.BreakHitResult` _outhit))
      (bind _returnvalue_3 (`KismetMathLibrary.Conv_VectorToRotator` _normal))
      (`GameplayStatics.SpawnDecalAttached` "/Game/Materials/M_Impact_Decal.M_Impact_Decal" (5.0 5.0 5.0) _hitcomponent "None" _location _returnvalue_3)
      (`GameplayStatics.SpawnEmitterAtLocation` (select `EPhysicalSurface` (`PhysicalMaterial.SurfaceType` _physmat) :!type "ParticleSystem Object Reference") _location _returnvalue_3)
      (message `/Game/VirtualRealityBP/Blueprints/PickupActorInterface.AddImpulse` _hitactor (* _returnvalue 1000.0))
      (`GameplayStatics.ApplyDamage` _hitactor 10.0))))

(fn `IsGun?`
  (returns (yes :type Boolean))
  (return true))

(fn `UserConstructionScript`)