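; BP_Lantern_2 is a VR pickup lantern actor that the motion controller can grab and release.
; Pickup disables physics on the LanternAxe component, attaches the root to the given component, moves it to a small relative offset and sets IsHeld.
; Drop restores physics, detaches the actor and clears IsHeld.
; An IsGun query returns false, marking it as a non-weapon item.
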(event `/Game/VRTemplate/VirtualRealityBP/Blueprints/PickupActorInterface.Pickup`
  (params (AttachTo :type "SceneComponent Object Reference"))
  (bind _returnvalue (`self.K2_GetRootComponent`))
  (`KismetSystemLibrary.PrintString` "picked up lantern")
  (`PrimitiveComponent.SetSimulatePhysics` (`self.LanternAxe`) false)
  (`SceneComponent.K2_AttachToComponent` _returnvalue AttachTo "None" "KeepWorld" "KeepWorld" "KeepWorld" false)
  (`KismetSystemLibrary.MoveComponentTo` _returnvalue (-4.0 0.0 -1.0))
  (set `self.IsHeld` true))

(event `/Game/VRTemplate/VirtualRealityBP/Blueprints/PickupActorInterface.Drop`
  (`PrimitiveComponent.SetSimulatePhysics` (`self.LanternAxe`) true)
  (`self.K2_DetachFromActor` "KeepWorld" "KeepWorld" "KeepWorld")
  (set `self.IsHeld` false))

(fn `IsGun?`
  (returns (yes :type Boolean))
  (return false))

(fn `UserConstructionScript`)