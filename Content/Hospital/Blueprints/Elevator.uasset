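; Hospital elevator Blueprint that animates a pair of sliding doors and moves the elevator vertically in response to the player.
; The player pawn entering DoorTrigger plays a timeline that slides both door meshes along local Y.
; Leaving the trigger chains three timelines through their Finished pins: a door slide, the elevator's Z travel, then another door slide.
; Timelines only use Play, with no reverse or restart, so the sequence has no return trip.
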(event `self.DoorTrigger.OnComponentBeginOverlap`
  (params (OverlappedComponent :type "PrimitiveComponent Object Reference") (OtherActor :type "Actor Object Reference") (OtherComp :type "PrimitiveComponent Object Reference") (OtherBodyIndex :type Integer) (bFromSweep :type Boolean) (SweepResult :type "HitResult Structure (by ref)"))
  (if (== OtherActor (`GameplayStatics.GetPlayerPawn` 0))
    (bind (_direction _newtrack_0 _newtrack_1) (`Timeline|DoorLocation`)
      (:`Update`
        (`SceneComponent.K2_SetRelativeLocation` (`self.SM_door`) (`KismetMathLibrary.MakeVector` -31.0 _newtrack_0) false false)
        (`SceneComponent.K2_SetRelativeLocation` (`self.SM_door1`) (`KismetMathLibrary.MakeVector` -31.0 _newtrack_1) false false)))))

(event `self.DoorTrigger.OnComponentEndOverlap`
  (params (OverlappedComponent :type "PrimitiveComponent Object Reference") (OtherActor :type "Actor Object Reference") (OtherComp :type "PrimitiveComponent Object Reference") (OtherBodyIndex :type Integer))
  (if (== OtherActor (`GameplayStatics.GetPlayerPawn` 0))
    (bind (_direction _newtrack_0 _newtrack_1) (`Timeline|Timeline_0`)
      (:`Update`
        (`SceneComponent.K2_SetRelativeLocation` (`self.SM_door`) (`KismetMathLibrary.MakeVector` -31.0 _newtrack_0) false false)
        (`SceneComponent.K2_SetRelativeLocation` (`self.SM_door1`) (`KismetMathLibrary.MakeVector` -31.0 _newtrack_1) false false))
      (:`Finished`
        (bind (_direction_2 _newtrack_0_2) (`Timeline|EleLocation`)
          (:`Update`
            (`SceneComponent.K2_SetRelativeLocation` (`self.Elevator`) (`KismetMathLibrary.MakeVector` 0.0 0.0 _newtrack_0_2) false false))
          (:`Finished`
            (bind (_direction_3 _newtrack_0_3 _newtrack_1_2) (`Timeline|Timeline_1`)
              (:`Update`
                (`SceneComponent.K2_SetRelativeLocation` (`self.SM_door`) (`KismetMathLibrary.MakeVector` -31.0 _newtrack_0_3) false false)
                (`SceneComponent.K2_SetRelativeLocation` (`self.SM_door1`) (`KismetMathLibrary.MakeVector` -31.0 _newtrack_1_2) false false)))))))))

(fn `UserConstructionScript`)