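; Hospital door actor that rotates open when the player pawn enters its trigger and rotates back when the pawn leaves.
; A world X comparison between actor and player picks one of two timelines, each driving the Door's relative roll.
; On exit the same comparison reverses the opposite side's timeline, so closing correctly assumes the player walked through the doorway.
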(event `self.Trigger.OnComponentBeginOverlap`
  (params (OverlappedComponent :type "PrimitiveComponent Object Reference") (OtherActor :type "Actor Object Reference") (OtherComp :type "PrimitiveComponent Object Reference") (OtherBodyIndex :type Integer) (bFromSweep :type Boolean) (SweepResult :type "HitResult Structure (by ref)"))
  (bind _returnvalue_x (`KismetMathLibrary.BreakVector` (`self.K2_GetActorLocation`)))
  (bind _returnvalue (`GameplayStatics.GetPlayerPawn` 0))
  (bind _door (`self.Door`))
  (bind _returnvalue_x_2 (`KismetMathLibrary.BreakVector` (`self.K2_GetActorLocation` _returnvalue)))
  (if (== OtherActor _returnvalue)
    (if (<= (- _returnvalue_x _returnvalue_x_2) 0.0)
      (bind (_direction _doorrotation) (`Timeline|DoorRotationController` :!label _label)
        (:`Update`
          (`SceneComponent.K2_SetRelativeRotation` _door (`KismetMathLibrary.MakeRotator` _doorrotation) false false)))
      (else
        (bind (_direction_2 _doorrotation_2) (`Timeline|Timeline_0` :!label _label_2)
          (:`Update`
            (`SceneComponent.K2_SetRelativeRotation` _door (`KismetMathLibrary.MakeRotator` _doorrotation_2) false false)))))))

(event `self.Trigger.OnComponentEndOverlap`
  (params (OverlappedComponent :type "PrimitiveComponent Object Reference") (OtherActor :type "Actor Object Reference") (OtherComp :type "PrimitiveComponent Object Reference") (OtherBodyIndex :type Integer))
  (bind _returnvalue (`GameplayStatics.GetPlayerPawn` 0))
  (bind _returnvalue_x (`KismetMathLibrary.BreakVector` (`self.K2_GetActorLocation`)))
  (bind _returnvalue_x_2 (`KismetMathLibrary.BreakVector` (`self.K2_GetActorLocation` _returnvalue)))
  (if (== OtherActor _returnvalue)
    (if (<= (- _returnvalue_x _returnvalue_x_2) 0.0)
      (goto _label_2 :!via `Reverse`)
      (else
        (goto _label :!via `Reverse`)))))

(fn `UserConstructionScript`)